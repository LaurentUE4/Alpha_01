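; Base interactable pickup actor that the player can collect into their inventory.
; A sphere trigger registers and unregisters the item with PlayerChar_BP on overlap, and the construction script sets mesh scale and trigger radius from variables.
; Interaction checks inventory space and item weight, sends ItemInfo to the interactor, then destroys the actor.
; SetHighlight toggles custom depth rendering and the widget's visibility.
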(event OnComponentBeginOverlap(InteractRadius)
  (params (OverlappedComponent :type Primitive%20Component%20Object%20Reference) (OtherActor :type Actor%20Object%20Reference) (OtherComp :type Primitive%20Component%20Object%20Reference) (OtherBodyIndex :type Integer) (bFromSweep :type Boolean) (SweepResult :type Hit%20Result%20Structure%20%28by%20ref%29))
  (bind _asplayer_char_bp (Utilities|Casting|CastToPlayerChar_BP OtherActor))
  (Class|InteractBPI|RegisterInteractable(Message) _asplayer_char_bp self))

(event OnComponentEndOverlap(InteractRadius)
  (params (OverlappedComponent :type Primitive%20Component%20Object%20Reference) (OtherActor :type Actor%20Object%20Reference) (OtherComp :type Primitive%20Component%20Object%20Reference) (OtherBodyIndex :type Integer))
  (bind _asplayer_char_bp (Utilities|Casting|CastToPlayerChar_BP OtherActor))
  (Class|InteractBPI|UnregisterInteractable(Message) _asplayer_char_bp self))

(event EventInteraction
  (params (Interactor :type Player%20Char%20BP%20Object%20Reference))
  (bind _iteminfo (Variables|Default|GetItemInfo))
  (if (Default|HasSpaceinInventory Interactor)
    (bind _poidsok_ (Default|CheckPoidsInventaire Interactor (Utilities|Struct|BreakItem_Info _iteminfo)))
    (if _poidsok_
      (Class|InteractBPI|PickUp(Message) Interactor _iteminfo)
      (Actor|DestroyActor))))

(fn ConstructionScript
  (Transformation|SetWorldScale3D (Variables|Default|GetInteractObject) (Variables|ItemTransform|GetMeshInteractScale))
  (Components|Sphere|SetSphereRadius (Variables|Default|GetInteractRadius) (Variables|ItemTransform|GetTriggerInteractSize) true))

(fn SetHighlight
  (params (Highlight? :type Boolean))
  (bind _widget (Variables|Default|GetWidget))
  (bind _returnvalue (UserInterface|GetUserWidgetObject _widget))
  (Rendering|SetRenderCustomDepth (Variables|Default|GetInteractObject) Highlight?)
  (if Highlight?
    (Widget|SetVisibility _returnvalue "Visible")
    (else
      (Widget|SetVisibility _returnvalue "Hidden"))))
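; Clock actor whose second, minute and hour hands rotate to simulate passing time.
; Tick feeds a chain of three latent Delays that ignore re-triggers while pending, stepping each hand at roughly second, minute and hour intervals.
; Each step adds a fixed yaw increment to the hand's relative rotation, with no reading of system or game time.
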(event EventBeginPlay)

(event Collision|EventActorBeginOverlap
  (params (OtherActor :type Actor%20Object%20Reference)))

(event EventTick
  (params (DeltaSeconds :type Float%20%28single-precision%29))
  (bind _heuresh (Variables|Default|GetHeuresH))
  (bind _secondesh (Variables|Default|GetSecondesH))
  (bind _minutesh (Variables|Default|GetMinutesH))
  (bind _relativerotation (Variables|/Script/Engine.SceneComponent|GetRelativeRotation _heuresh))
  (bind _relativerotation_2 (Variables|/Script/Engine.SceneComponent|GetRelativeRotation _secondesh))
  (bind _relativerotation_3 (Variables|/Script/Engine.SceneComponent|GetRelativeRotation _minutesh))
  (Utilities|FlowControl|Delay 1.0)
  (Transformation|SetRelativeRotation _secondesh (Math|Rotator|MakeRotator (.roll _relativerotation_2) (.pitch _relativerotation_2) (+ (.yaw _relativerotation_2) 6.0)) false false)
  (Utilities|FlowControl|Delay 59.0)
  (Transformation|SetRelativeRotation _minutesh (Math|Rotator|MakeRotator (.roll _relativerotation_3) (.pitch _relativerotation_3) (+ (.yaw _relativerotation_3) 6.0)) false false)
  (Utilities|FlowControl|Delay 3599.0)
  (Transformation|SetRelativeRotation _heuresh (Math|Rotator|MakeRotator (.roll _relativerotation) (.pitch _relativerotation) (+ (.yaw _relativerotation) 3e+01)) false false))

(fn ConstructionScript)